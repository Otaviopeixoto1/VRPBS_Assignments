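; Character Blueprint that plays a procedural walk animation on arm and leg joint components.
; On BeginPlay it enables player input, and each press of the space bar toggles the walk on or off.
; While walking, Tick sets each joint's relative roll from a sine of real time scaled by speed and amplitude.
; Opposite arm and leg swing together, with the other pair mirrored by negating the angle.
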(event `self.ReceiveBeginPlay`
  (`self.EnableInput` (`GameplayStatics.GetPlayerController` 0)))

(event `Key|SpaceBar` :consume false
  (params (Key :type "Key Structure"))
  (:`Pressed`
    (`/Engine/EditorBlueprintResources/StandardMacros.FlipFlop`
      (:`A`
        (set `self.WalkActive` true))
      (:`B`
        (set `self.WalkActive` false)))))

(event `self.ReceiveTick`
  (params (DeltaSeconds :type "Float (single-precision)"))
  (bind _returnvalue (* (`KismetMathLibrary.Sin` (* (`self.AnimationSpeed`) (`GameplayStatics.GetRealTimeSeconds`))) (`self.RotationAmplitude`)))
  (if (`self.WalkActive`)
    (`SceneComponent.K2_SetRelativeRotation` (`self.RLegJoint`) (`KismetMathLibrary.MakeRotator` _returnvalue) false false)
    (`SceneComponent.K2_SetRelativeRotation` (`self.LArmJoint`) (`KismetMathLibrary.MakeRotator` _returnvalue) false false)
    (`SceneComponent.K2_SetRelativeRotation` (`self.LLegJoint`) (`KismetMathLibrary.MakeRotator` (* _returnvalue -1.0)) false false)
    (`SceneComponent.K2_SetRelativeRotation` (`self.RArmJoint`) (`KismetMathLibrary.MakeRotator` (* _returnvalue -1.0)) false false)))

(fn `UserConstructionScript`)