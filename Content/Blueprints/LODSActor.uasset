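; Actor that implements its own screen-size LOD by swapping its static mesh between high, mid and low versions.
; Each Tick it projects points on the mesh's bounding box, built from the Offsets array, through the first PlayerController, clamped to the viewport.
; The larger width or height fraction of the resulting screen rectangle is compared against LowThr and HighThr to pick the mesh.
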(event `self.ReceiveBeginPlay`
  (`StaticMeshComponent.SetStaticMesh` (`self.meshComponent`) (`self.meshHigh`)))

(event `self.ReceiveTick`
  (params (DeltaSeconds :type "Float (single-precision)"))
  (bind _lowthr (`self.lowThr`))
  (bind _highthr (`self.highThr`))
  (bind (_x _y) (`KismetMathLibrary.BreakVector2D` (`WidgetLayoutLibrary.GetViewportSize`)))
  (bind (_origin _boxextent) (`KismetSystemLibrary.GetComponentBounds` (`self.meshComponent`)))
  (bind (_x_2 _y_2) (`KismetMathLibrary.BreakVector2D` (`WidgetLayoutLibrary.GetViewportSize`)))
  (bind _returnvalue (`KismetMathLibrary.FMax` (/ (- (`self.MaxBoundsX`) (`self.MinBoundsX`)) _x) (/ (- (`self.MaxBoundsY`) (`self.MinBoundsY`)) _y)))
  (bind _outactors (`GameplayStatics.GetAllActorsOfClass` "/Script/Engine.PlayerController"))
  (for (_array_element _array_index) (`self.Offsets`)
    (if (== _array_index 0)
      (bind (_x_3 _y_3) (`KismetMathLibrary.BreakVector2D` (`GameplayStatics.ProjectWorldToScreen` (`|GetArrayItem` _outactors) (+ _origin (* _array_element _boxextent)))))
      (bind _returnvalue_2 (`KismetMathLibrary.FMin` (`KismetMathLibrary.FMax` _x_3) _x_2))
      (set `self.MaxBoundsX` _returnvalue_2)
      (set `self.MinBoundsX` _returnvalue_2)
      (bind _returnvalue_3 (`KismetMathLibrary.FMin` (`KismetMathLibrary.FMax` _y_3) _y_2))
      (set `self.MaxBoundsY` _returnvalue_3)
      (set `self.MinBoundsY` _returnvalue_3)
      (else
        (set `self.MaxBoundsX` (`KismetMathLibrary.FMax` (`self.MaxBoundsX`) _returnvalue_2))
        (set `self.MinBoundsX` (`KismetMathLibrary.FMin` _returnvalue_2 (`self.MinBoundsX`)))
        (set `self.MaxBoundsY` (`KismetMathLibrary.FMax` (`self.MaxBoundsY`) _returnvalue_3))
        (set `self.MinBoundsY` (`KismetMathLibrary.FMin` _returnvalue_3 (`self.MinBoundsY`))))))
  (if (and (>= _returnvalue 0.0) (< _returnvalue _lowthr))
    (`StaticMeshComponent.SetStaticMesh` (`self.meshComponent`) (`self.meshLow`))
    (elif (and (> _returnvalue _lowthr) (< _returnvalue _highthr))
      (`StaticMeshComponent.SetStaticMesh` (`self.meshComponent`) (`self.meshMid`))
      (elif (>= _returnvalue _highthr)
        (`StaticMeshComponent.SetStaticMesh` (`self.meshComponent`) (`self.meshHigh`))))))

(fn `UserConstructionScript`)